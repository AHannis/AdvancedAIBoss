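; BP_Enemy_Ranged is a rifle-wielding enemy built on a parent enemy class, overriding its attack, movement speeds and ideal combat range.
; On BeginPlay it spawns a weapon actor, attaches it to the hand rifle socket and signals that it is equipped.
; Attack plays a montage whose notify has BPCAttacks fire a damaging bullet trace from weapon to target, then ends the attack on completion or interruption.
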(event `self.ReceiveBeginPlay`
  (`parent.ReceiveBeginPlay`)
  (`self.EquipWeapon`))

(event `self.EquipWeapon`
  ;[1 1 1] Equip Weapon
  (bind _returnvalue (`|SpawnActorFromClass` null (`KismetMathLibrary.MakeTransform` (0.0 0.0 0.0)) "Undefined" "MultiplyWithRoot" null null))
  (bind _output_get (set `self.WeaponActor` _returnvalue))
  (`self.K2_AttachToComponent` _output_get (`self.Mesh`) "hand_r_rifle_socket" "SnapToTarget" "SnapToTarget" "SnapToTarget" true)
  (set `self.IsWieldingWeapon` true)
  (`self.OnWeaponEquipped`))

(event `self.Attack`
  (params (AttackTarget :type "Actor Object Reference"))
  ;[1 1 1] Fire Rifle
  (`parent.Attack` AttackTarget)
  (bind _notifyname (`|PlayMontage` (`self.Mesh`))
    (:`OnCompleted`
      (`self.AttackEnd` AttackTarget :!label _label))
    (:`OnInterrupted`
      (goto _label))
    (:`OnNotifyBegin`
      (switch `name` _notifyname
        (:`Fire`
          (`self.FireBullet` (`self.BPC_Attacks`) (`self.K2_GetActorLocation` (`self.WeaponActor`)) (`self.K2_GetActorLocation` AttackTarget) (make `` 10.0 0 0 false true)))))))

(fn `GetIdealRange`
  (returns (AttackRadius :type "Float (double-precision)") (DefendRadius :type "Float (double-precision)"))
  (return 600.0 600.0))

(fn `SetMovementSpeed`
  (params (Speed :type Byte :default 0))
  (returns (SpeedValue :type "Float (double-precision)"))
  (bind _output_get (set `CharacterMovementComponent.MaxWalkSpeed` (select `byte` Speed :`NewEnumerator0` 0.0 :`NewEnumerator1` 200.0 :`NewEnumerator2` 300.0 :`NewEnumerator3` 500.0 :!type "Float (single-precision)") (`self.CharacterMovement`)))
  (return _output_get))

(fn `UserConstructionScript`
  (`parent.UserConstructionScript`))